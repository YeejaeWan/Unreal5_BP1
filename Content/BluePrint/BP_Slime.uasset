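; BP_Slime is a slime actor that slides forward along world X, apparently racing toward an arrival point.
; Tick moves it without sweep by delta time times a speed re-rolled every frame, so its pace jitters.
; Overlapping any actor sets Arrived, which this graph never reads, while the OnArrived dispatcher fires at BeginPlay with itself rather than on overlap.
; A name-printing node is left disconnected.
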(event EventBeginPlay
  (Default|CallOnArrived self))

(event Collision|EventActorBeginOverlap
  (params (OtherActor :type Actor%20Object%20Reference))
  (Variables|Default|SetbArrived true))

(event EventTick
  (params (DeltaSeconds :type Float%20%28single-precision%29))
  (Transformation|SetActorLocation (+ (Transformation|GetActorLocation) (Math|Vector|MakeVector (* DeltaSeconds (Math|Random|RandomFloatinRange 5e+02 2e+03)) 0.0 0.0)) false false))

(fn ConstructionScript)